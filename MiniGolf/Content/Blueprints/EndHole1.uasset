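; EndHole1 is the trigger actor that ends a hole in the mini golf game when a golfball overlaps it.
; It caches the MiniGolf game mode on BeginPlay.
; On overlap it destroys the ball, plays a 2D sound, then after a short delay increments the game mode's current hole and clears its HoleSetup flag.
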(event EventBeginPlay
  (bind _asmini_golf_game_mode (Utilities|Casting|CastToMiniGolf_GameMode (Game|GetGameMode)))
  (Variables|Default|SetGameMode _asmini_golf_game_mode))

(event Collision|EventActorBeginOverlap
  (params (OtherActor :type Actor%20Object%20Reference))
  (bind _gamemode (Variables|Default|GetGameMode))
  (bind _asgolfball (Utilities|Casting|CastToGolfball OtherActor))
  (Actor|DestroyActor _asgolfball)
  (Audio|PlaySound2D "/Game/golfball.golfball" 1.0 1.0 0.0 0 0)
  (Utilities|FlowControl|Delay 1.0)
  (Variables|/Game/Blueprints/MiniGolf_GameMode.MiniGolf_GameMode_C|SetCurrentHole _gamemode (+ (Variables|/Game/Blueprints/MiniGolf_GameMode.MiniGolf_GameMode_C|GetCurrentHole _gamemode) 1))
  (Variables|/Game/Blueprints/MiniGolf_GameMode.MiniGolf_GameMode_C|SetHoleSetup _gamemode false))

(fn ConstructionScript)