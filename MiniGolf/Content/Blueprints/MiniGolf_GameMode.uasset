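; Game mode for a nine-hole mini golf game that holds the current hole, per-hole scores and game state flags.
; On BeginPlay, StartGame clears the GameWon and HoleSetup flags, sets the first hole and zeroes every hole score.
; Every Tick, a switch on CurrentHole copies that hole's score into CurrentScore.
; Nothing in this file changes scores or advances holes after the reset.
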(event EventBeginPlay
  (Utilities|StartGame))

(event EventTick
  (params (DeltaSeconds :type Float%20%28single-precision%29))
  (switch int (Variables|Default|GetCurrentHole)
    (:1
      (Variables|Default|SetCurrentScore (Variables|Default|GetHole1Score)))
    (:2
      (Variables|Default|SetCurrentScore (Variables|Default|GetHole2Score)))
    (:3
      (Variables|Default|SetCurrentScore (Variables|Default|GetHole3Score)))
    (:4
      (Variables|Default|SetCurrentScore (Variables|Default|GetHole4Score)))
    (:5
      (Variables|Default|SetCurrentScore (Variables|Default|GetHole5Score)))
    (:6
      (Variables|Default|SetCurrentScore (Variables|Default|GetHole6Score)))
    (:7
      (Variables|Default|SetCurrentScore (Variables|Default|GetHole7Score)))
    (:8
      (Variables|Default|SetCurrentScore (Variables|Default|GetHole8Score)))
    (:9
      (Variables|Default|SetCurrentScore (Variables|Default|GetHole9Score)))))

(fn ConstructionScript)