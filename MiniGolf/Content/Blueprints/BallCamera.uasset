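; Camera actor that keeps itself pointed at the golf ball.
; BeginPlay finds the Golfball actor in the level and caches the reference.
; Each Tick rotates the actor toward the ball's location, or searches for the ball again whenever the cached reference is invalid.
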(event EventBeginPlay
  (bind _returnvalue (Actor|GetActorOfClass "/Game/Blueprints/Golfball.Golfball_C"))
  (Variables|Default|SetBallReference _returnvalue))

(event Collision|EventActorBeginOverlap
  (params (OtherActor :type Actor%20Object%20Reference)))

(event EventTick
  (params (DeltaSeconds :type Float%20%28single-precision%29))
  (Utilities|IsValid (Variables|Default|GetBallReference)
    (:Is%20Valid
      (Transformation|SetActorRotation self (Math|Rotator|FindLookatRotation (Transformation|GetActorLocation self) (Transformation|GetActorLocation (Variables|Default|GetBallReference)))))
    (:Is%20Not%20Valid
      (bind _returnvalue (Actor|GetActorOfClass "/Game/Blueprints/Golfball.Golfball_C"))
      (Variables|Default|SetBallReference _returnvalue))))

(fn ConstructionScript)