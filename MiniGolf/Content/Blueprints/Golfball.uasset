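; Physics-driven golf ball that registers with the player character, enters play when hit by a Putter, and exposes a force-based Launch.
; Tick blends to the chase camera while it rolls in play, damping low speeds until it snaps to rest.
; Coming to rest unlocks and repositions the player, and the view blends back to the character.
; Destruction or an invalid Ball component resets the player's locks, charge, animation and camera.
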(event EventBeginPlay
  (bind _returnvalue (Actor|GetActorOfClass "/Game/Blueprints/BallCamera.BallCamera_C"))
  (Variables|Default|SetBallChaseCamera (Variables|/Game/Blueprints/BallCamera.BallCamera_C|GetBallCineCamera _returnvalue))
  (bind _returnvalue_2 (Actor|GetActorOfClass "/Game/Blueprints/ThirdPersonCharacter.ThirdPersonCharacter_C"))
  (Variables|/Game/Blueprints/ThirdPersonCharacter.ThirdPersonCharacter_C|SetBallReference _returnvalue_2 self)
  (Utilities|FlowControl|Delay 2.7)
  (Default|UpdatePlayerPos _returnvalue_2))

(event EventDestroyed
  (CallFunction|BeforeDestruction))

(event EventTick
  (params (DeltaSeconds :type Float%20%28single-precision%29))
  (bind _ball (Variables|Default|GetBall))
  (Utilities|IsValid (Variables|Default|GetBall)
    (:Is%20Valid
      (bind _returnvalue (Physics|GetPhysicsLinearVelocity (Variables|Default|GetBall) "None"))
      (bind _output_get (Variables|Default|SetIsRolling (>= (Math|Vector|VectorLength _returnvalue) 0.01)))
      (if _output_get
        (if (Variables|Default|GetInPlay)
          (Game|Player|SetViewTargetwithBlend (Game|GetPlayerController 0) (Components|GetOwner (Variables|Default|GetBallChaseCamera)) 0.7 "VTBlend_Linear" 0.0 false)
          (bind _returnvalue_2 (Physics|GetPhysicsLinearVelocity (Variables|Default|GetBall) "None"))
          (if (<= (Math|Vector|VectorLength _returnvalue_2) 0.09)
            (Physics|SetPhysicsLinearVelocity _ball "0, 0, 0" false "None")
            (Class|PrimitiveComponent|SetPhysicsAngularVelocityinDegrees _ball "0, 0, 0" false "None")
            (Variables|Default|SetInPlay false)
            (bind _returnvalue_3 (Actor|GetActorOfClass "/Game/Blueprints/ThirdPersonCharacter.ThirdPersonCharacter_C"))
            (Variables|/Game/Blueprints/ThirdPersonCharacter.ThirdPersonCharacter_C|SetLockPlayer _returnvalue_3 false)
            (Utilities|FlowControl|Delay 1.2)
            (Default|UpdatePlayerPos _returnvalue_3)
            (elif (<= (Math|Vector|VectorLength _returnvalue_2) 1e+01)
              (Physics|SetPhysicsLinearVelocity (Variables|Default|GetBall) (* _returnvalue_2 -0.05) true "None"))))
        (else
          (bind _returnvalue_4 (Actor|GetActorOfClass "/Game/Blueprints/ThirdPersonCharacter.ThirdPersonCharacter_C"))
          (Utilities|FlowControl|Delay 0.0)
          (Game|Player|SetViewTargetwithBlend (Game|GetPlayerController 0) _returnvalue_4 0.7 "VTBlend_Linear" 0.0 false))))
    (:Is%20Not%20Valid
      (CallFunction|BeforeDestruction))))

(event Collision|EventHit
  (params (MyComp :type Primitive%20Component%20Object%20Reference) (Other :type Actor%20Object%20Reference) (OtherComp :type Primitive%20Component%20Object%20Reference) (bSelfMoved :type Boolean) (HitLocation :type Vector :default "0, 0, 0") (HitNormal :type Vector :default "0, 0, 0") (NormalImpulse :type Vector :default "0, 0, 0") (Hit :type Hit%20Result%20Structure%20%28by%20ref%29))
  (Utilities|Casting|CastToPutter Other)
  (Variables|Default|SetInPlay true))

(fn ConstructionScript)

(fn Launch
  (params (LaunchVector :type Vector) (PowerFraction :type Float%20%28single-precision%29))
  (Physics|AddForce (Variables|Default|GetBall) (* LaunchVector PowerFraction) "None" false))

(fn BeforeDestruction
  (bind _returnvalue (Actor|GetActorOfClass "/Game/Blueprints/ThirdPersonCharacter.ThirdPersonCharacter_C"))
  (Variables|Default|SetInPlay false)
  (Variables|/Game/Blueprints/ThirdPersonCharacter.ThirdPersonCharacter_C|SetLockPlayer _returnvalue false)
  (Variables|/Game/Blueprints/ThirdPersonCharacter.ThirdPersonCharacter_C|SetLockPlayerMovement _returnvalue false)
  (Variables|/Game/Blueprints/ThirdPersonCharacter.ThirdPersonCharacter_C|SetPowerCharge _returnvalue 0.0)
  (Components|Animation|SetPosition (Variables|/Script/Engine.Character|GetMesh _returnvalue) 0.0 false)
  (Audio|Components|Audio|Stop (Variables|/Script/Engine.Character|GetMesh _returnvalue))
  (Game|Player|SetViewTargetwithBlend (Game|GetPlayerController 0) _returnvalue 0.0 "VTBlend_Linear" 0.0 false))