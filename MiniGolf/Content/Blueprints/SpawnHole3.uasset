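; Spawn point actor for hole 3 of a mini golf game that places a golf ball at its own location.
; It caches the MiniGolf game mode on BeginPlay and polls it every Tick.
; When the current hole is 3 and not yet set up, it spawns a scaled-down Golfball and sets the game mode's HoleSetup flag to prevent repeat spawns.
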(event EventTick
  (params (DeltaSeconds :type Float%20%28single-precision%29))
  (if (== (Variables|/Game/Blueprints/MiniGolf_GameMode.MiniGolf_GameMode_C|GetCurrentHole (Variables|Default|GetGameMode)) 3)
    (if (not (Variables|/Game/Blueprints/MiniGolf_GameMode.MiniGolf_GameMode_C|GetHoleSetup (Variables|Default|GetGameMode)))
      (Game|SpawnActorfromClass "/Game/Blueprints/Golfball.Golfball_C" (Math|Transform|MakeTransform (Transformation|GetActorLocation) "0, 0, 0" "0.035000,0.035000,0.035000") "Undefined" 0 0)
      (Variables|/Game/Blueprints/MiniGolf_GameMode.MiniGolf_GameMode_C|SetHoleSetup (Variables|Default|GetGameMode) true))))

(event EventBeginPlay
  (bind _asmini_golf_game_mode (Utilities|Casting|CastToMiniGolf_GameMode (Game|GetGameMode)))
  (Variables|Default|SetGameMode _asmini_golf_game_mode))

(fn ConstructionScript)