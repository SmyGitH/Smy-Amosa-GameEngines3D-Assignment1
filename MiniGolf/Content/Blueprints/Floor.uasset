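; Mini-golf floor that acts as an out-of-bounds surface, resetting any golf ball that hits it to the current hole's start point.
; BeginPlay caches the MiniGolf game mode and finds one spawn marker actor for each of the nine holes by class.
; On Hit, it destroys the Golfball and switches on the game mode's CurrentHole to spawn a new ball at that marker.
; Respawns use BallScale, except hole nine, which uses unit scale.
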(event EventBeginPlay
  (bind _asmini_golf_game_mode (Utilities|Casting|CastToMiniGolf_GameMode (Game|GetGameMode)))
  (Variables|Default|SetGameMode _asmini_golf_game_mode)
  (bind _returnvalue (Actor|GetActorOfClass "/Game/Blueprints/SpawnHole1.SpawnHole1_C"))
  (Variables|Default|Sethole1 _returnvalue)
  (bind _returnvalue_2 (Actor|GetActorOfClass "/Game/Blueprints/SpawnHole2.SpawnHole2_C"))
  (Variables|Default|Sethole2 _returnvalue_2)
  (bind _returnvalue_3 (Actor|GetActorOfClass "/Game/Blueprints/SpawnHole3.SpawnHole3_C"))
  (Variables|Default|Sethole3 _returnvalue_3)
  (bind _returnvalue_4 (Actor|GetActorOfClass "/Game/Blueprints/SpawnHole4.SpawnHole4_C"))
  (Variables|Default|Sethole4 _returnvalue_4)
  (bind _returnvalue_5 (Actor|GetActorOfClass "/Game/Blueprints/SpawnHole5.SpawnHole5_C"))
  (Variables|Default|Sethole5 _returnvalue_5)
  (bind _returnvalue_6 (Actor|GetActorOfClass "/Game/Blueprints/SpawnHole6.SpawnHole6_C"))
  (Variables|Default|Sethole6 _returnvalue_6)
  (bind _returnvalue_7 (Actor|GetActorOfClass "/Game/Blueprints/SpawnHole7.SpawnHole7_C"))
  (Variables|Default|Sethole7 _returnvalue_7)
  (bind _returnvalue_8 (Actor|GetActorOfClass "/Game/Blueprints/SpawnHole8.SpawnHole8_C"))
  (Variables|Default|Sethole8 _returnvalue_8)
  (bind _returnvalue_9 (Actor|GetActorOfClass "/Game/Blueprints/SpawnHole9.SpawnHole9_C"))
  (Variables|Default|Sethole9 _returnvalue_9))

(event EventTick
  (params (DeltaSeconds :type Float%20%28single-precision%29)))

(event Collision|EventHit
  (params (MyComp :type Primitive%20Component%20Object%20Reference) (Other :type Actor%20Object%20Reference) (OtherComp :type Primitive%20Component%20Object%20Reference) (bSelfMoved :type Boolean) (HitLocation :type Vector :default "0, 0, 0") (HitNormal :type Vector :default "0, 0, 0") (NormalImpulse :type Vector :default "0, 0, 0") (Hit :type Hit%20Result%20Structure%20%28by%20ref%29))
  (bind _asgolfball (Utilities|Casting|CastToGolfball Other))
  (Actor|DestroyActor _asgolfball)
  (switch int (Variables|/Game/Blueprints/MiniGolf_GameMode.MiniGolf_GameMode_C|GetCurrentHole (Variables|Default|GetGameMode))
    (:1
      ;[1 1 1] Comment
      (Game|SpawnActorfromClass "/Game/Blueprints/Golfball.Golfball_C" (Math|Transform|MakeTransform (Transformation|GetActorLocation (Variables|Default|Gethole1)) "0, 0, 0" (Variables|Default|GetBallScale)) "Undefined" 0 0))
    (:2
      (Game|SpawnActorfromClass "/Game/Blueprints/Golfball.Golfball_C" (Math|Transform|MakeTransform (Transformation|GetActorLocation (Variables|Default|Gethole2)) "0, 0, 0" (Variables|Default|GetBallScale)) "Undefined" 0 0))
    (:3
      (Game|SpawnActorfromClass "/Game/Blueprints/Golfball.Golfball_C" (Math|Transform|MakeTransform (Transformation|GetActorLocation (Variables|Default|Gethole3)) "0, 0, 0" (Variables|Default|GetBallScale)) "Undefined" 0 0))
    (:4
      (Game|SpawnActorfromClass "/Game/Blueprints/Golfball.Golfball_C" (Math|Transform|MakeTransform (Transformation|GetActorLocation (Variables|Default|Gethole4)) "0, 0, 0" (Variables|Default|GetBallScale)) "Undefined" 0 0))
    (:5
      (Game|SpawnActorfromClass "/Game/Blueprints/Golfball.Golfball_C" (Math|Transform|MakeTransform (Transformation|GetActorLocation (Variables|Default|Gethole5)) "0, 0, 0" (Variables|Default|GetBallScale)) "Undefined" 0 0))
    (:6
      (Game|SpawnActorfromClass "/Game/Blueprints/Golfball.Golfball_C" (Math|Transform|MakeTransform (Transformation|GetActorLocation (Variables|Default|Gethole6)) "0, 0, 0" (Variables|Default|GetBallScale)) "Undefined" 0 0))
    (:7
      (Game|SpawnActorfromClass "/Game/Blueprints/Golfball.Golfball_C" (Math|Transform|MakeTransform (Transformation|GetActorLocation (Variables|Default|Gethole7)) "0, 0, 0" (Variables|Default|GetBallScale)) "Undefined" 0 0))
    (:8
      (Game|SpawnActorfromClass "/Game/Blueprints/Golfball.Golfball_C" (Math|Transform|MakeTransform (Transformation|GetActorLocation (Variables|Default|Gethole8)) "0, 0, 0" (Variables|Default|GetBallScale)) "Undefined" 0 0))
    (:9
      (Game|SpawnActorfromClass "/Game/Blueprints/Golfball.Golfball_C" (Math|Transform|MakeTransform (Transformation|GetActorLocation (Variables|Default|Gethole9))) "Undefined" 0 0))))

(fn ConstructionScript)